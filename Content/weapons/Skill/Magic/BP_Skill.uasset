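; BP_Skill is a skeletal skill actor for the magic weapon system, owned by a BP_Magic.
; Spell, EndSpell and OffEquipped are empty events, apparently hooks for child skills.
; OnEquipped re-enables movement and sets the idle state through the owning BP_Magic.
; Helper functions resolve the owner chain by casting the owner to BP_Magic, then that magic's owner to Character.
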(event `Spell`)

(event `EndSpell`)

(event `OnEquipped`
  (bind _newparam (`self.GetOwner toMagic`))
  (`/Game/weapons/BP_Weapon.SetCanMove` _newparam true)
  (`/Game/weapons/BP_Weapon.SetStateIdling` _newparam))

(event `OffEquipped`)

(fn `GetOwner toMagic`
  (returns (NewParam :type "/Game/weapons/Skill/Magic/BP_Magic Object Reference"))
  (bind _asbp_magic (cast `/Game/weapons/Skill/Magic/BP_Magic` (`self.GetOwner`)))
  (return _asbp_magic))

(fn `GetOwnerToCharacter`
  (returns (AsCharacter :type "Character Object Reference"))
  (bind _ascharacter (cast `Character` (`self.GetOwner` (`self.GetOwner toMagic`))))
  (return _ascharacter))

(fn `UserConstructionScript`)