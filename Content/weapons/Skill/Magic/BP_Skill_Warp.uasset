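; Warp magic skill that teleports its owning character to the point under the mouse cursor.
; While equipped, Tick traces WorldStatic objects under the cursor to place a preview mesh and surface-aligned decal.
; Spell stores the hit location, locks movement and plays the warp montage, or ends the attack on a miss.
; A separate Warp event performs the teleport at a fixed height, and EndSpell restores movement.
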(event `self.ReceiveBeginPlay`
  (`parent.ReceiveBeginPlay`)
  (`SceneComponent.SetVisibility` (`self.StaticMesh`) false false)
  (`SceneComponent.SetVisibility` (`self.Decal`) false false))

(event `self.ReceiveTick`
  (params (DeltaSeconds :type "Float (single-precision)"))
  (bind _decal (`self.Decal`))
  (`parent.ReceiveTick` DeltaSeconds)
  (if (`self.Equipped`)
    (bind (_location _impactnormal) (`self.GetCursorLocation`)
      (:`True`
        (`SceneComponent.K2_SetWorldLocation` _decal _location false false)
        (`SceneComponent.K2_SetWorldLocation` (`self.StaticMesh`) _location false false)
        (`SceneComponent.K2_SetWorldRotation` _decal (`KismetMathLibrary.Conv_VectorToRotator` _impactnormal) false false)
        (`SceneComponent.SetVisibility` _decal true false)
        (`SceneComponent.SetVisibility` (`self.StaticMesh`) true false))
      (:`False`
        (`SceneComponent.SetVisibility` (`self.Decal`) false false :!label _label)
        (`SceneComponent.SetVisibility` (`self.StaticMesh`) false false)))
    (else
      (goto _label))))

(event `self.Spell`
  (`parent.Spell`)
  (bind _location (`self.GetCursorLocation`)
    (:`True`
      (set `self.WarpLocation` _location)
      (set `self.CanWarp` true)
      (`/Game/weapons/BP_Weapon.SetCanMove` (`self.GetOwner toMagic`) false)
      (`Character.PlayAnimMontage` (`self.GetOwnerToCharacter`) "/Game/Character/Montages/SkillMotion/MG_Warp_Montage.MG_Warp_Montage" 1.0 "None"))
    (:`False`
      (`/Game/weapons/BP_Weapon.EndAttack` (`self.GetOwner toMagic`))
      (set `self.CanWarp` false))))

(event `self.EndSpell`
  (`parent.EndSpell`)
  (`/Game/weapons/BP_Weapon.SetCanMove` (`self.GetOwner toMagic`) true))

(event `Warp`
  (if (`self.CanWarp`)
    (set `self.CanWarp` false)
    (`self.K2_SetActorLocation` (`self.GetOwnerToCharacter`) (`KismetMathLibrary.MakeVector` (.x (`self.WarpLocation`)) (.y (`self.WarpLocation`)) 200.0) false true)))

(event `self.OnEquipped`
  (`parent.OnEquipped`)
  (set `self.Equipped` true))

(event `self.OffEquipped`
  (`parent.OffEquipped`)
  (set `self.Equipped` false))

(fn `UserConstructionScript`
  (`parent.UserConstructionScript`))