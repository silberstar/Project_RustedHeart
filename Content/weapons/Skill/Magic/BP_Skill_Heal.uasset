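; BP_Skill_Heal is a magic skill Blueprint that heals its caster.
; On Spell, it runs the parent logic, enables movement on the owner's magic object and plays a buff montage on the owning character.
; It then increases health by a fixed amount through the character's StatusComponent, if one exists.
; EndSpell calls the parent and enables movement again.
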(event `self.ReceiveBeginPlay`
  (`parent.ReceiveBeginPlay`))

(event `self.Spell`
  (bind _ascharacter (`self.GetOwnerToCharacter`))
  (bind _returnvalue (`self.GetComponentByClass` _ascharacter "/Game/Conponents/StatusComponent.StatusComponent_C"))
  (`parent.Spell`)
  (`/Game/weapons/BP_Weapon.SetCanMove` (`self.GetOwner toMagic`) true)
  (`Character.PlayAnimMontage` _ascharacter "/Game/Character/Montages/SkillMotion/MG_Buff_Montage.MG_Buff_Montage" 1.0 "None")
  (`/Engine/EditorBlueprintResources/StandardMacros.IsValid` _returnvalue
    (:`Is Valid`
      (`/Game/Conponents/StatusComponent.IncreaseHealth` _returnvalue 30.0))))

(event `self.EndSpell`
  (`parent.EndSpell`)
  (`/Game/weapons/BP_Weapon.SetCanMove` (`self.GetOwner toMagic`) true))

(fn `UserConstructionScript`
  (`parent.UserConstructionScript`))