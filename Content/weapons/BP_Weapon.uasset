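; Base weapon actor with empty equip, attack and end-attack hooks, presumably for child weapons to fill in.
; It queries and sets the owner's state through I_State and reads combat type through I_Weapon, allowing attacks only when the type matches and the owner is idle.
; SendDamage damages only Characters other than the owner, crediting the owner's controller.
; Simple events toggle transformation, refill ammo on reload and re-enable shooting.
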(event `OnEquipped`)

(event `OnUnEquipped`)

(event `WeaponTransformation`
  (set `self.Transform` true))

(event `WeaponTransformationRevers`
  (set `self.Transform` false))

(event `Reload`
  (set `self.Ammo` (`self.MaxAmmo`)))

(event `Shot`
  (set `self.CanShooting` true))

(fn `Attack`)

(fn `CanAttack`
  (returns (ReturnValue :type Boolean))
  (return (and (`|EnumEquality` (`self.CombatType`) (`self.GetCombatType`)) (`self.IsStateIdling`))))

(fn `EndAttack`)

(fn `GetCombatType`
  (returns (OutCombatType :type "/Game/Enums/E_CombatStyle Enum"))
  (bind _returnvalue (`self.GetOwner`))
  (if (`KismetSystemLibrary.DoesImplementInterface` _returnvalue "/Game/Interfaces/I_Weapon.I_Weapon_C")
    (bind _outcombattype (message `/Game/Interfaces/I_Weapon.GetCombatType` _returnvalue))
    (return _outcombattype)))

(fn `IsStateIdling`
  (returns (Result :type Boolean))
  (bind _returnvalue (`self.GetOwner`))
  (if (`KismetSystemLibrary.DoesImplementInterface` _returnvalue "/Game/Interfaces/I_State.I_State_C")
    (bind _result (message `/Game/Interfaces/I_State.IsStateIdling` _returnvalue))
    (return _result)))

(fn `SendDamage`
  (params (OtherActor :type "Actor Object Reference") (Damage :type "Float (double-precision)" :default 1.0))
  (returns (Result :type Boolean))
  (if (!= OtherActor (`self.GetOwner`))
    (cast `Character` (`local.OtherActor`)
      (:`then`
        (`GameplayStatics.ApplyDamage` OtherActor Damage (`self.GetInstigatorController` (`self.GetOwner`)) self)
        (return true))
      (:`CastFailed`
        _)))
  (return false))

(fn `SetAttacking`
  (bind _returnvalue (`self.GetOwner`))
  (if (`KismetSystemLibrary.DoesImplementInterface` _returnvalue "/Game/Interfaces/I_State.I_State_C")
    (message `/Game/Interfaces/I_State.SetStateAttacking` _returnvalue)))

(fn `SetCanMove`
  (params (InCanMove :type Boolean))
  (bind _returnvalue (`self.GetOwner`))
  (if (`KismetSystemLibrary.DoesImplementInterface` _returnvalue "/Game/Interfaces/I_State.I_State_C")
    (message `/Game/Interfaces/I_State.SetCanMove` _returnvalue (`local.InCanMove`))))

(fn `SetStateIdling`
  (bind _returnvalue (`self.GetOwner`))
  (if (`KismetSystemLibrary.DoesImplementInterface` _returnvalue "/Game/Interfaces/I_State.I_State_C")
    (message `/Game/Interfaces/I_State.SetStateIdling` _returnvalue)))

(fn `SetStateSpelling`
  (bind _returnvalue (`self.GetOwner`))
  (if (`KismetSystemLibrary.DoesImplementInterface` _returnvalue "/Game/Interfaces/I_State.I_State_C")
    (message `/Game/Interfaces/I_State.SetStateSpelling` _returnvalue)))

(fn `UserConstructionScript`)