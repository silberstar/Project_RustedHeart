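; Unarmed melee weapon that turns the owning character's punches and kicks into combo-based damage.
; On BeginPlay it attaches four hit collisions to fist and kick sockets on the owner's mesh, then disables its sphere colliders.
; OnCollision enables the requested limb's collider, and OffCollision disables them all.
; Overlaps send damage from WeaponDamageComponent for the current combo count, and attack start and end events notify that component.
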(event `self.ReceiveBeginPlay`
  (`parent.ReceiveBeginPlay`)
  (`PrimitiveComponent.SetCollisionEnabled` (`self.LeftPunch`) "NoCollision")
  (`|ExecutionSequence`
    (:`then_0`
      (`self.AttachCollisionToSoket` (`self.LeftPunch`) "Fist_L")
      (`self.AttachCollisionToSoket` (`self.RightPunch`) "Fist_R"))
    (:`then_1`
      (`self.AttachCollisionToSoket` (`self.LeftKick`) "Kick_L")
      (`self.AttachCollisionToSoket` (`self.RightKick`) "Kick_R"))
    (:`then_2`
      (`self.SetAllCollisions` "NoCollision"))))

(event `self.OnCollision`
  (params (FistCollision :type "/Game/Enums/E_FistCOllisionType Enum" :default "NewEnumerator0"))
  (`parent.OnCollision` FistCollision)
  (switch `/Game/Enums/E_FistCOllisionType` FistCollision
    (:`NewEnumerator1`
      (`PrimitiveComponent.SetCollisionEnabled` (`self.LeftPunch`) "QueryAndPhysics"))
    (:`NewEnumerator2`
      (`PrimitiveComponent.SetCollisionEnabled` (`self.RightPunch`) "QueryAndPhysics"))
    (:`NewEnumerator3`
      (`PrimitiveComponent.SetCollisionEnabled` (`self.LeftKick`) "QueryAndPhysics"))
    (:`NewEnumerator4`
      (`PrimitiveComponent.SetCollisionEnabled` (`self.RightKick`) "QueryAndPhysics"))))

(event `self.OffCollision`
  (`parent.OffCollision`)
  (`self.SetAllCollisions` "NoCollision"))

(event `self.LeftPunch.OnComponentBeginOverlap`
  (params (OverlappedComponent :type "PrimitiveComponent Object Reference") (OtherActor :type "Actor Object Reference") (OtherComp :type "PrimitiveComponent Object Reference") (OtherBodyIndex :type Integer) (bFromSweep :type Boolean) (SweepResult :type "HitResult Structure (by ref)"))
  (bind _returnvalue (`/Game/Conponents/WeaponDamageComponent.GetComboDamage` (`self.WeaponDamageComponent`) (`self.ComboCount`)))
  (`self.SendDamage` OtherActor _returnvalue))

(event `self.RightPunch.OnComponentBeginOverlap`
  (params (OverlappedComponent :type "PrimitiveComponent Object Reference") (OtherActor :type "Actor Object Reference") (OtherComp :type "PrimitiveComponent Object Reference") (OtherBodyIndex :type Integer) (bFromSweep :type Boolean) (SweepResult :type "HitResult Structure (by ref)"))
  (bind _returnvalue (`/Game/Conponents/WeaponDamageComponent.GetComboDamage` (`self.WeaponDamageComponent`) (`self.ComboCount`)))
  (`self.SendDamage` OtherActor _returnvalue))

(event `self.LeftKick.OnComponentBeginOverlap`
  (params (OverlappedComponent :type "PrimitiveComponent Object Reference") (OtherActor :type "Actor Object Reference") (OtherComp :type "PrimitiveComponent Object Reference") (OtherBodyIndex :type Integer) (bFromSweep :type Boolean) (SweepResult :type "HitResult Structure (by ref)"))
  (bind _returnvalue (`/Game/Conponents/WeaponDamageComponent.GetComboDamage` (`self.WeaponDamageComponent`) (`self.ComboCount`)))
  (`self.SendDamage` OtherActor _returnvalue))

(event `self.RightKick.OnComponentBeginOverlap`
  (params (OverlappedComponent :type "PrimitiveComponent Object Reference") (OtherActor :type "Actor Object Reference") (OtherComp :type "PrimitiveComponent Object Reference") (OtherBodyIndex :type Integer) (bFromSweep :type Boolean) (SweepResult :type "HitResult Structure (by ref)"))
  (bind _returnvalue (`/Game/Conponents/WeaponDamageComponent.GetComboDamage` (`self.WeaponDamageComponent`) (`self.ComboCount`)))
  (`self.SendDamage` OtherActor _returnvalue))

(event `CustomEvent`
  (`parent.StartCombo`)
  (`/Game/Conponents/WeaponDamageComponent.StartAttack` (`self.WeaponDamageComponent`)))

(event `CustomEvent_1`
  (`parent.EndAttack`)
  (`/Game/Conponents/WeaponDamageComponent.EndAttack` (`self.WeaponDamageComponent`)))

(fn `AttachCollisionToSoket`
  (params (Collision :type "SphereComponent Object Reference") (SoketName :type Name))
  (bind _ascharacter (cast `Character` (`self.GetOwner`)))
  (`SceneComponent.K2_AttachToComponent` Collision (`Character.Mesh` _ascharacter) SoketName "KeepRelative" "KeepRelative" "KeepRelative" true))

(fn `SetAllCollisions`
  (params (CollisionEnabledType :type "ECollisionEnabled Enum" :default "NoCollision"))
  (for _array_element (`self.K2_GetComponentsByClass` "/Script/Engine.SphereComponent")
    (`PrimitiveComponent.SetCollisionEnabled` _array_element (`local.CollisionEnabledType`))))

(fn `UserConstructionScript`)