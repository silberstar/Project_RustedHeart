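; Enemy character that carries holstered weapons, takes damage with hit reactions and dies into a ragdoll.
; BeginPlay spawns a greatsword and two longswords on holster sockets, hides those not matching WeaponStyle, and creates dynamic body materials.
; AnyDamage updates health and its widget, turns toward the attacker, then either shows damage-source-specific particles or knockback, or ragdolls and destroys itself after a delay.
; State and weapon functions delegate attacks to the current weapon.
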(event `self.ReceiveBeginPlay`
  (`|ExecutionSequence`
    (:`then_0`
      (bind _returnvalue (`|SpawnActorFromClass` "/Game/weapons/Melee/Sword/BP_GreateSword.BP_GreateSword_C" (`KismetMathLibrary.MakeTransform` (0.0 0.0 0.0)) "Undefined" "OverrideRootScale" self null))
      (bind _output_get (set `self.GrateSword` _returnvalue))
      (`self.K2_AttachToComponent` _output_get (`self.Mesh`) "Holster_GreateSword" "KeepRelative" "KeepRelative" "KeepRelative" true)
      (if (!= (`self.WeaponStyle`) 0)
        (`self.SetActorHiddenInGame` _output_get true)))
    (:`then_1`
      (bind _returnvalue_2 (`|SpawnActorFromClass` "/Game/weapons/Melee/Sword/BP_LongSword1.BP_LongSword1_C" (`KismetMathLibrary.MakeTransform` (0.0 0.0 0.0)) "Undefined" "OverrideRootScale" self null))
      (bind _output_get_2 (set `self.LongSword1` _returnvalue_2))
      (`self.K2_AttachToComponent` _output_get_2 (`self.Mesh`) "Holster_TwoHended" "KeepRelative" "KeepRelative" "KeepRelative" true)
      (if (!= (`self.WeaponStyle`) 1)
        (`self.SetActorHiddenInGame` _output_get_2 true)
        (`self.SetActorHiddenInGame` (`/Game/weapons/Melee/Sword/BP_LongSword1.Sword` _output_get_2) true)))
    (:`then_2`
      (bind _returnvalue_3 (`|SpawnActorFromClass` "/Game/weapons/Melee/Sword/BP_LongSword1.BP_LongSword1_C" (`KismetMathLibrary.MakeTransform` (0.0 0.0 0.0)) "Undefined" "OverrideRootScale" self null))
      (`PrimitiveComponent.SetCollisionEnabled` (`self.Mesh`) "QueryAndPhysics")
      (bind _output_get_3 (set `self.LongSword2` _returnvalue_3))
      (`self.K2_AttachToComponent` _output_get_3 (`self.Mesh`) "Holster_Sword" "KeepRelative" "KeepRelative" "KeepRelative" true)
      (if (!= (`self.WeaponStyle`) 2)
        (`self.SetActorHiddenInGame` (`/Game/weapons/Melee/Sword/BP_LongSword1.Sword` _output_get_3) true)
        (`self.SetActorHiddenInGame` _output_get_3 true)))
    (:`then_3`
      (`|ExecutionSequence`
        (:`then_0`
          (bind _returnvalue_4 (`KismetMaterialLibrary.CreateDynamicMaterialInstance` "/Game/Character/Materials/M_UE4Man_Body_Inst.M_UE4Man_Body_Inst"))
          (`KismetArrayLibrary.Array_Add` (`self.DynamicMaterials`) _returnvalue_4)
          (bind _returnvalue_5 (`KismetMaterialLibrary.CreateDynamicMaterialInstance` "/Game/Character/Materials/M_UE4Man_ChestLogo_Inst.M_UE4Man_ChestLogo_Inst"))
          (`KismetArrayLibrary.Array_Add` (`self.DynamicMaterials`) _returnvalue_5))
        (:`then_1`
          (`PrimitiveComponent.SetMaterial` (`self.Mesh`) 0 (`|GetArrayItem` (`self.DynamicMaterials`)))
          (`PrimitiveComponent.SetMaterial` (`self.Mesh`) 1 (`|GetArrayItem` (`self.DynamicMaterials`) 1)))))
    (:`then_4`
      (`self.UpdateHealth`)
      (`SceneComponent.SetVisibility` (`self.HealthWidget`) false false))))

(event `self.ReceiveAnyDamage`
  (params (Damage :type "Float (single-precision)") (DamageType :type "DamageType Object Reference") (InstigatedBy :type "Controller Object Reference") (DamageCauser :type "Actor Object Reference"))
  (bind _couser (`self.Couser`))
  (bind _emberprticle (`self.EmberPrticle`))
  (bind _electricprticle (`self.ElectricPrticle`))
  (set `self.Couser` DamageCauser)
  (bind _ascharacter (cast `Character` (`Controller.K2_GetPawn` InstigatedBy)))
  (set `self.Attacker` _ascharacter)
  (bind _output_get (set `self.Damage` Damage))
  (`/Game/Conponents/StatusComponent.DecreaseHealth` (`self.StatusComponent`) _output_get)
  (`self.UpdateHealth`)
  (`self.PlayAnimMontage` "/Game/Character/Montages/MeleeMotion/HitReaction_Montage.HitReaction_Montage")
  (set `self.StateType` "NewEnumerator8")
  (`NavMovementComponent.StopMovementKeepPathing` (`self.CharacterMovement`))
  (`self.K2_SetActorRotation` (`KismetMathLibrary.FindLookAtRotation` (`self.K2_GetActorLocation`) (`self.K2_GetActorLocation` (`self.Attacker`))))
  (`self.SetBodyColor` (struct :`R` 1.0 :`A` 1.0))
  (`KismetSystemLibrary.Delay` 0.1)
  (`self.SetBodyColor` (`self.BodyColor`))
  (if (`/Game/Conponents/StatusComponent.isDead` (`self.StatusComponent`))
    (if (`|EnumInequality` (`self.StateType`) "NewEnumerator4")
      (set `self.StateType` "NewEnumerator4")
      (`self.Ragdoll`)
      (`KismetSystemLibrary.RetriggerableDelay` 3.0)
      (`self.Dead`))
    (else
      (`SceneComponent.SetVisibility` (`self.HealthWidget`) true false)
      (bind _asbp_magic (cast `/Game/weapons/Skill/Magic/BP_Magic` _couser)
        (:`then`
          (bind _asbp_skill_throw (cast `/Game/weapons/Skill/Magic/BP_Skill_Throw` (`/Game/weapons/Skill/Magic/BP_Magic.CurrentSkill` _asbp_magic)))
          (switch `int` (`/Game/weapons/Skill/Magic/BP_Skill_Throw.CurrentItem` _asbp_skill_throw)
            (:`0`
              (`ActorComponent.SetActive` _emberprticle true false)
              (`KismetSystemLibrary.Delay` 2.0)
              (`ActorComponent.SetActive` _emberprticle false false))
            (:`1`
              (`ActorComponent.SetActive` _electricprticle true false)
              (`KismetSystemLibrary.Delay` 2.0)
              (`ActorComponent.SetActive` _electricprticle false false))))
        (:`CastFailed`
          (bind _asbp_melee (cast `/Game/weapons/Melee/BP_Melee` _couser))
          (cast `/Game/weapons/Melee/Sword/BP_LongSword1` _asbp_melee
            (:`then`
              (`self.Launch` -20.0))
            (:`CastFailed`
              (cast `/Game/weapons/Melee/Knuckle/BP_Fist` (`self.Couser`))
              (`self.Launch` 1.0))))))))

(event `Dead`
  (`self.K2_DestroyActor` (`self.GrateSword`))
  (`self.K2_DestroyActor` (`self.LongSword1`))
  (`self.K2_DestroyActor` (`self.LongSword2`))
  (`self.K2_DestroyActor`))

(event `Attack`
  (bind _currentweapon (`self.CurrentWeapon`)
    (:`then`
      (`/Game/weapons/BP_Weapon.Attack` _currentweapon))
    (:`else`)))

(fn `Attach`)

(fn `Detach`)

(fn `Equipped`
  (set `self.StateType` "NewEnumerator0"))

(fn `GetCombatType`
  (returns (OutCombatType :type "/Game/Enums/E_CombatStyle Enum"))
  (return (`self.CombatType`)))

(fn `GetCurrentWeapon`
  (returns (CurrentWeapon :type "/Game/weapons/BP_Weapon Object Reference"))
  (return (`self.CurrentWeapon`)))

(fn `Hited`
  (returns (Result :type Boolean))
  (set `self.StateType` "NewEnumerator0")
  (return false))

(fn `IsStateAttacking`
  (returns (Result :type Boolean))
  (return (`|EnumEquality` (`self.StateType`) "NewEnumerator3")))

(fn `IsStateIdling`
  (returns (Result :type Boolean))
  (return (`|EnumEquality` (`self.StateType`) "NewEnumerator0")))

(fn `Launch`
  (params (Value :type "Float (double-precision)"))
  (`self.K2_AddActorWorldOffset` (* (`KismetMathLibrary.Normal` (`self.GetActorForwardVector`)) (`local.Value`))))

(fn `Ragdoll`
  (bind _mesh (`self.Mesh`))
  (`PrimitiveComponent.SetCollisionEnabled` (`self.CapsuleComponent`) "NoCollision")
  (set `SkeletalMeshComponent.GlobalAnimRateScale` 0.0 _mesh)
  (`PrimitiveComponent.SetSimulatePhysics` _mesh true)
  (`PrimitiveComponent.SetCollisionEnabled` _mesh "QueryAndPhysics")
  (`PrimitiveComponent.AddForce` _mesh (* (* (`KismetMathLibrary.GetDirectionUnitVector` (`self.K2_GetActorLocation` (`self.Attacker`)) (`self.K2_GetActorLocation`)) (`self.Damage`)) 250000.0) "None" false))

(fn `SetBodyColor`
  (params (LBodyColor :type "LinearColor Structure"))
  (for _array_element (`self.DynamicMaterials`)
    (`MaterialInstanceDynamic.SetVectorParameterValue` :`self` _array_element :`ParameterName` "BodyColor")))

(fn `SetCanMove`
  (params (InCanMove :type Boolean))
  (returns (Result :type Boolean))
  (return false))

(fn `SetCurrentWeapon`
  (params (NewWeapon :type "/Game/weapons/BP_Weapon Object Reference"))
  (returns (Weapon :type "/Game/weapons/BP_Weapon Object Reference"))
  (bind _newweapon (`local.NewWeapon`))
  (`/Engine/EditorBlueprintResources/StandardMacros.IsValid` (`self.CurrentWeapon`)
    (:`Is Valid`
      (`/Game/weapons/BP_Weapon.OnUnEquipped` (`self.CurrentWeapon`)))
    (:`Is Not Valid`
      _))
  (`/Engine/EditorBlueprintResources/StandardMacros.IsValid` _newweapon
    (:`Is Valid`
      (bind _output_get (set `self.CurrentWeapon` _newweapon))
      (`/Game/weapons/BP_Weapon.OnEquipped` _output_get)
      (return _output_get))
    (:`Is Not Valid`
      (set `self.CurrentWeapon` null)
      (return null))))

(fn `SetStateAttacking`
  (returns (Result :type Boolean))
  (set `self.StateType` "NewEnumerator3")
  (return false))

(fn `SetStateIdling`
  (returns (Result :type Boolean))
  (set `self.StateType` "NewEnumerator0")
  (return false))

(fn `SetStateSpelling`
  (returns (Result :type Boolean))
  (return false))

(fn `UnEquipped`
  (set `self.StateType` "NewEnumerator0"))

(fn `UpdateHealth`
  (bind _statuscomponent (`self.StatusComponent`))
  (bind _aswb_health_bar (cast `/Game/Widgets/WB_HealthBar` (`WidgetComponent.GetUserWidgetObject` (`self.HealthWidget`))))
  (`/Game/Widgets/WB_HealthBar.UpdateHealthBar` _aswb_health_bar (`/Game/Conponents/StatusComponent.Health` _statuscomponent) (`/Game/Conponents/StatusComponent.MaxHealth` _statuscomponent)))

(fn `UserConstructionScript`
  (`TextRenderComponent.K2_SetText` (`self.PawnName`) (`KismetTextLibrary.Conv_StringToText` (`KismetSystemLibrary.GetDisplayName` self))))

(fn `WeaponAttach`
  (returns (NewParam :type Boolean))
  (`self.Attach`)
  (return false))

(fn `WeaponDetach`
  (returns (NewParam :type Boolean))
  (`self.Detach`)
  (return false))

(fn `WeaponEquipped`
  (returns (NewParam :type Boolean))
  (`self.Equipped`)
  (return false))

(fn `WeaponUnEquipped`
  (returns (NewParam :type Boolean))
  (`self.UnEquipped`)
  (return false))