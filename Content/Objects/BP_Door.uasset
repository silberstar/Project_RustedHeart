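; BP_Door is a two-panel door that opens while the player is in its trigger.
; DoorTriger overlaps with BP_Player play the DoorOpen timeline on entry and reverse it on exit.
; Timeline outputs drive the relative locations of RightDoor and LeftDoor, both offset from RightDoor's starting location cached at BeginPlay.
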(event `self.ReceiveBeginPlay`
  (bind _returnvalue_location (`KismetMathLibrary.BreakTransform` (`SceneComponent.GetRelativeTransform` (`self.RightDoor`))))
  (set `self.newvar` _returnvalue_location))

(event `self.DoorTriger.OnComponentBeginOverlap`
  (params (OverlappedComponent :type "PrimitiveComponent Object Reference") (OtherActor :type "Actor Object Reference") (OtherComp :type "PrimitiveComponent Object Reference") (OtherBodyIndex :type Integer) (bFromSweep :type Boolean) (SweepResult :type "HitResult Structure (by ref)"))
  (bind _newvar (`self.newvar`))
  (cast `/Game/Player/BP_Player` OtherActor)
  (bind (_direction _doorright _leftdoor) (`Timeline|DoorOpen` :!label _label)
    (:`Update`
      (`SceneComponent.K2_SetRelativeLocation` (`self.RightDoor`) (+ _doorright _newvar) false false)
      (`SceneComponent.K2_SetRelativeLocation` (`self.LeftDoor`) (+ _leftdoor _newvar) false false))))

(event `self.DoorTriger.OnComponentEndOverlap`
  (params (OverlappedComponent :type "PrimitiveComponent Object Reference") (OtherActor :type "Actor Object Reference") (OtherComp :type "PrimitiveComponent Object Reference") (OtherBodyIndex :type Integer))
  (cast `/Game/Player/BP_Player` OtherActor)
  (goto _label :!via `Reverse`))

(fn `UserConstructionScript`)